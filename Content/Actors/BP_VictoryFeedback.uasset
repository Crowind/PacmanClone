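; Victory feedback actor that plays audio and drives an expanding material effect centered on the player when victory is triggered.
; The Victory event sends the PacPerson's location to the static mesh materials, unpauses the audio paused at BeginPlay, and enables updating.
; Each Tick then grows a radius by a fixed multiplier and writes it to the material's VictoryRadius parameter, producing frame-rate-dependent exponential growth.
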(event EventBeginPlay
  (Class|AudioComponent|SetPaused (Variables|Default|GetVictoryAudioComponent) true))

(event Collision|EventActorBeginOverlap
  (params (OtherActor :type Actor%20Object%20Reference)))

(event EventTick
  (params (DeltaSeconds :type Float%20%28single-precision%29))
  (if (Variables|Default|GetUpdate)
    (bind _output_get (Variables|Default|SetRadius (* (Variables|Default|GetRadius) 1.12)))
    (Rendering|Material|SetScalarParameterValueonMaterials (Variables|Default|GetStaticMesh) "VictoryRadius" _output_get)))

(event EventVictory
  (CallFunction|Victory1))

(fn ConstructionScript)

(fn Victory1
  (bind _returnvalue (Actor|GetActorOfClass "/Script/PacmanClone.PacPerson"))
  (Rendering|Material|SetVectorParameterValueonMaterials (Variables|Default|GetStaticMesh) "PlayerPosition" (Transformation|GetActorLocation _returnvalue))
  (Variables|Default|SetUpdate true)
  (Class|AudioComponent|SetPaused (Variables|Default|GetVictoryAudioComponent) false))