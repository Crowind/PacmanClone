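; Pac-Man-style character Blueprint that handles the visuals on top of movement state read through getters.
; Each tick it advances a material time parameter while movement is active, sets material rotation from movement direction, and repositions a direction indicator mesh to match the displayed direction.
; Init events reset appearance and then enable movement.
; PlayDeath calls the parent, then swaps to a death material stamped with start time and facing, so animation is material-driven.
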(event EventBeginPlay)

(event Collision|EventActorBeginOverlap
  (params (OtherActor :type Actor%20Object%20Reference)))

(event EventTick
  (params (DeltaSeconds :type Float%20%28single-precision%29))
  (bind _mesh (Variables|Character|GetMesh))
  (bind _displaydirectionmesh (Variables|Default|GetDisplayDirectionMesh))
  (Utilities|FlowControl|Sequence
    (:then_0
      (bind _returnvalue (Class|PacMazePawn|GetPacMovementActive))
      (if _returnvalue
        (bind _output_get (Variables|Default|SetEatingTime (+ DeltaSeconds (Variables|Default|GetEatingTime))))
        (Rendering|Material|SetScalarParameterValueonMaterials (Variables|Character|GetMesh) "PacTime" _output_get)))
    (:then_1
      (bind _returnvalue_2 (Class|PacMazePawn|GetMovementDirection))
      (switch Utilities|FlowControl|Switch|SwitchonEMazeDirection _returnvalue_2
        (:Down
          (Rendering|Material|SetScalarParameterValueonMaterials _mesh "Rotation" 0.75))
        (:Right
          (Rendering|Material|SetScalarParameterValueonMaterials _mesh "Rotation" 0.0))
        (:Up
          (Rendering|Material|SetScalarParameterValueonMaterials _mesh "Rotation" 0.25))
        (:Left
          (Rendering|Material|SetScalarParameterValueonMaterials _mesh "Rotation" 0.5))))
    (:then_2
      (bind _returnvalue_3 (Class|PacMazePawn|GetDisplayedDirection))
      (switch Utilities|FlowControl|Switch|SwitchonEMazeDirection _returnvalue_3
        (:Down
          (Transformation|SetRelativeRotation _displaydirectionmesh "0, 0, 0" false false)
          (Transformation|SetRelativeLocation _displaydirectionmesh "0,50.000000, 0" false true))
        (:Right
          (Transformation|SetRelativeRotation _displaydirectionmesh "0,-90.000000, 0" false false)
          (Transformation|SetRelativeLocation _displaydirectionmesh "50.000000,0.000000, 0" false true))
        (:Up
          (Transformation|SetRelativeRotation _displaydirectionmesh "0,180.000000, 0" false false)
          (Transformation|SetRelativeLocation _displaydirectionmesh "0,-50.000000, 0" false true))
        (:Left
          (Transformation|SetRelativeRotation _displaydirectionmesh "0,90.000000, 0" false false)
          (Transformation|SetRelativeLocation _displaydirectionmesh "-50.000000, 0, 0" false true))))))

(event EventInitPacPerson
  (Class|PacMazePawn|SetPacMovementActive true))

(event EventInitPacPersonAppereance
  (Rendering|Material|SetMaterial (Variables|Character|GetMesh) 0 (Variables|Default|GetMazeMaterial))
  (Class|PacMazePawn|SetPacMovementActive false)
  (Class|PacMazePawn|SetMovementDirection "Left")
  (Class|PacMazePawn|SetDisplayDirection "Left")
  (Variables|Default|SetEatingTime 0.0))

(event EventPlayDeath
  (bind _mesh (Variables|Character|GetMesh))
  (|CallParentFunction)
  (Rendering|Material|SetMaterial (Variables|Character|GetMesh) 0 (Variables|Default|GetDeathMaterial))
  (Rendering|Material|SetScalarParameterValueonMaterials _mesh "StartTime" (Utilities|Time|GetTimeSeconds))
  (bind _returnvalue (Class|PacMazePawn|GetMovementDirection))
  (switch Utilities|FlowControl|Switch|SwitchonEMazeDirection _returnvalue
    (:Down
      (Rendering|Material|SetScalarParameterValueonMaterials _mesh "Rotation" 0.75))
    (:Right
      (Rendering|Material|SetScalarParameterValueonMaterials _mesh "Rotation" 0.0))
    (:Up
      (Rendering|Material|SetScalarParameterValueonMaterials _mesh "Rotation" 0.25))
    (:Left
      (Rendering|Material|SetScalarParameterValueonMaterials _mesh "Rotation" 0.5))))

(fn ConstructionScript)