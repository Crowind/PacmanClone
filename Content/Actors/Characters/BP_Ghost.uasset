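; Ghost enemy character for a Pac-Man-style game, driven by a behavior tree through its GhostAiController.
; On BeginPlay it assigns itself to its start node, runs the behavior tree, then seeds the blackboard.
; The blackboard receives scatter and eaten destinations from referenced actors, the BP_PacPerson found in the level as player, a fixed frightened duration, and matching default and current ghost states.
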(event EventBeginPlay
  (Class|PacMazeZone|Assign (Variables|Default|GetStartNode) self)
  (bind _asghost_ai_controller (Utilities|Casting|CastToGhostAiController (Pawn|GetController)))
  (AI|RunBehaviorTree _asghost_ai_controller (Variables|Default|GetBTAsset))
  (CallFunction|InitGhostBlackboardValues _asghost_ai_controller))

(event Collision|EventActorBeginOverlap
  (params (OtherActor :type Actor%20Object%20Reference)))

(event EventTick
  (params (DeltaSeconds :type Float%20%28single-precision%29)))

(fn ConstructionScript)

(fn InitGhostBlackboardValues
  (params (Controller :type Ghost%20Ai%20Controller%20Object%20Reference))
  (bind _returnvalue (AI|GetBlackboard Controller))
  (Utilities|FlowControl|Sequence
    (:then_0
      (AI|Components|Blackboard|SetValueasVector _returnvalue (LocalVariables|GetScatteringDestinationKey) (Transformation|GetActorLocation (Variables|Default|GetScatteringDestination))))
    (:then_1
      (bind _returnvalue_2 (Actor|GetActorOfClass "/Game/Actors/Characters/BP_PacPerson.BP_PacPerson_C"))
      (AI|Components|Blackboard|SetValueasObject _returnvalue (LocalVariables|GetPlayerKey) _returnvalue_2))
    (:then_2
      (AI|Components|Blackboard|SetValueasVector _returnvalue (LocalVariables|GetEatenDestinationKey) (Transformation|GetActorLocation (Variables|Default|GetEatenDestination))))
    (:then_3
      (AI|Components|Blackboard|SetValueasFloat _returnvalue (LocalVariables|GetFrightenedDurationKey) 1e+01))
    (:then_4
      (AI|Components|Blackboard|SetValueasEnum _returnvalue (LocalVariables|GetDefaultPacGhostStateKey) 1))
    (:then_5
      (AI|Components|Blackboard|SetValueasEnum _returnvalue (LocalVariables|GetCurrentPacGhostStateKey) 1))))