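; BP_Inky is the Inky ghost character in a Pac-Man game, specializing a parent ghost class's initialization.
; InitGhost sets DotsThreshold to a fixed value on respawn, otherwise to Inky's default from PacmanGameMode, then runs the parent initialization.
; It finally writes a Blinky reference into the GhostAiController's blackboard, making that ghost available to Inky's AI.
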(event EventBeginPlay
  (|CallParentFunction))

(event Collision|EventActorBeginOverlap
  (params (OtherActor :type Actor%20Object%20Reference))
  (|CallParentFunction OtherActor) ; This node is disabled and will not be called.\nDrag off pins to build functionality.
)

(event EventTick
  (params (DeltaSeconds :type Float%20%28single-precision%29))
  (|CallParentFunction DeltaSeconds) ; This node is disabled and will not be called.\nDrag off pins to build functionality.
)

(event EventInitGhost
  (params (respawn :type Boolean))
  (Utilities|FlowControl|Sequence
    (:then_0
      (if respawn
        (Variables|Default|SetDotsThreshold 17)
        (else
          (bind _aspacman_game_mode (Utilities|Casting|CastToPacmanGameMode (Game|GetGameMode)))
          (bind _returnvalue (Class|PacmanGameMode|GetInkyDotsDefaultThreshold _aspacman_game_mode))
          (Variables|Default|SetDotsThreshold _returnvalue))))
    (:then_1
      (|CallParentFunction respawn))
    (:then_2
      (bind _asghost_ai_controller (Utilities|Casting|CastToGhostAiController (Pawn|GetController)))
      (AI|Components|Blackboard|SetValueasObject (AI|GetBlackboard _asghost_ai_controller) (Variables|Default|GetBlinkyKey) (Variables|Default|GetBlinky)))))

(fn ConstructionScript
  (|CallParentFunction))