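; BP_Pinky is the Pinky ghost character, a child Blueprint that leaves nearly all behavior to its parent class.
; It overrides InitGhost to set DotsThreshold before calling the parent, using a higher threshold on respawn and zero otherwise.
; BeginPlay, Tick and the construction script only forward to the parent.
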(event EventBeginPlay
  (|CallParentFunction))

(event Collision|EventActorBeginOverlap
  (params (OtherActor :type Actor%20Object%20Reference))
  (|CallParentFunction OtherActor) ; This node is disabled and will not be called.\nDrag off pins to build functionality.
)

(event EventTick
  (params (DeltaSeconds :type Float%20%28single-precision%29))
  (|CallParentFunction DeltaSeconds))

(event EventInitGhost
  (params (respawn :type Boolean))
  (Utilities|FlowControl|Sequence
    (:then_0
      (if respawn
        (Variables|Default|SetDotsThreshold 7)
        (else
          (Variables|Default|SetDotsThreshold 0))))
    (:then_1
      (|CallParentFunction respawn))))

(fn ConstructionScript
  (|CallParentFunction))