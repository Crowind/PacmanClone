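; BP_PlayerStartPacNode is a Pac maze node that, judging by its name, marks the player's start position.
; On BeginPlay it runs the parent logic, then finds actors tagged "Player" and passes each one that casts to PacMazePawn into Assign.
; Assign is not defined in this graph, and the construction script only calls its parent.
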(event EventBeginPlay
  (|CallParentFunction)
  (bind _outactors (Actor|GetAllActorswithTag "Player"))
  (for _array_element _outactors
    (bind _aspac_maze_pawn (Utilities|Casting|CastToPacMazePawn _array_element))
    (Class|PacMazeZone|Assign _aspac_maze_pawn)))

(event Collision|EventActorBeginOverlap
  (params (OtherActor :type Actor%20Object%20Reference))
  (|CallParentFunction OtherActor) ; This node is disabled and will not be called.\nDrag off pins to build functionality.
)

(event EventTick
  (params (DeltaSeconds :type Float%20%28single-precision%29))
  (|CallParentFunction DeltaSeconds) ; This node is disabled and will not be called.\nDrag off pins to build functionality.
)

(fn ConstructionScript
  (|CallParentFunction))