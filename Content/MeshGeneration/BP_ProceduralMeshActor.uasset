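; An actor Blueprint that builds a three-section procedural mesh when play begins.
; After the parent BeginPlay, it creates each section on the ProceduralMesh component from one shared vertex array and that section's own triangle and UV arrays.
; The same material is applied to all three sections, and the construction script is empty.
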(event EventBeginPlay
  (bind _material (Variables|Default|GetMaterial))
  (bind _proceduralmesh (Variables|Default|GetProceduralMesh))
  (|CallParentFunction)
  (Utilities|FlowControl|Sequence
    (:then_0
      (Class|ProceduralMeshComponent|CreateMeshSectionLinearColor _proceduralmesh 0 (Variables|Default|GetVertices) (Variables|Default|GetTriangles1) 0 (Variables|Default|GetUVs1) 0 0 0 0 0 false)
      (Rendering|Material|SetMaterial _proceduralmesh 0 _material))
    (:then_1
      (Class|ProceduralMeshComponent|CreateMeshSectionLinearColor _proceduralmesh 1 (Variables|Default|GetVertices) (Variables|Default|GetTriangles2) 0 (Variables|Default|GetUVs2) 0 0 0 0 0 false)
      (Rendering|Material|SetMaterial _proceduralmesh 1 _material))
    (:then_2
      (Class|ProceduralMeshComponent|CreateMeshSectionLinearColor _proceduralmesh 2 (Variables|Default|GetVertices) (Variables|Default|GetTriangles3) 0 (Variables|Default|GetUVs3) 0 0 0 0 0 false)
      (Rendering|Material|SetMaterial _proceduralmesh 2 _material))))

(event Collision|EventActorBeginOverlap
  (params (OtherActor :type Actor%20Object%20Reference)))

(event EventTick
  (params (DeltaSeconds :type Float%20%28single-precision%29)))

(fn ConstructionScript)